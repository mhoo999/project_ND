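; BP_Trowable_Brick is a throwable brick item that launches as a projectile.
; Its Throw event runs once, detaches the brick from its parent while keeping the world transform, then applies the given velocity and activates its ProjectileMovementComponent.
; BeginPlay only runs a short delay with nothing after it, and a forward-vector throw remains disconnected.
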(event `self.ReceiveBeginPlay`
  (`KismetSystemLibrary.Delay` 0.2))

(event `Throw`
  (params (Velocity :type "Vector Structure"))
  (bind _projectilemovementcomponent (`self.ProjectileMovementComponent`))
  (`/Engine/EditorBlueprintResources/StandardMacros.DoOnce` false
    (:`Completed`
      (`self.K2_DetachFromActor` "KeepWorld" "KeepWorld" "KeepWorld")
      (`|ExecutionSequence`
        (:`then_0`
          (set `MovementComponent.Velocity` Velocity _projectilemovementcomponent)
          (`ActorComponent.SetActive` _projectilemovementcomponent true true))))))

(fn `UserConstructionScript`)