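; Player character Blueprint that handles basic locomotion and camera look through Enhanced Input.
; BeginPlay casts the controller to NDPlayerController and adds the IMC_NDPlayer mapping context.
; Input actions drive movement relative to control rotation, inverted-Y pitch, yaw and jumping.
; Sprint (hold) and walk (toggle) both set MaxWalkSpeed directly, so ending a sprint restores default speed even when walk is toggled on.
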(event `self.ReceiveBeginPlay`
  (bind _asndplayer_controller (cast `NDPlayerController` (`self.GetController`)))
  (bind _returnvalue (pcsubsystem `EnhancedInputLocalPlayerSubsystem` _asndplayer_controller))
  (`/Engine/EditorBlueprintResources/StandardMacros.IsValid` _returnvalue
    (:`Is Valid`
      (`EnhancedInputSubsystemInterface.AddMappingContext` _returnvalue "/Game/Project_ND/Character/Player_Input/IMC_NDPlayer.IMC_NDPlayer" 0 (struct)))))

(event `EnhancedInput|/Game/Project_ND/Character/Player_Input/IA_NDMove`
  (params (ActionValue :type "Vector2D Structure") (ElapsedSeconds :type "Float (double-precision)") (TriggeredSeconds :type "Float (double-precision)") (InputAction :type "InputAction Object Reference" :default "/Game/Project_ND/Character/Player_Input/IA_NDMove.IA_NDMove"))
  (bind _returnvalue (`self.GetControlRotation`))
  (:`Triggered`
    (`self.AddMovementInput` (`KismetMathLibrary.GetRightVector` _returnvalue) ActionValue_X)
    (`self.AddMovementInput` (`KismetMathLibrary.GetForwardVector` _returnvalue) ActionValue_Y)))

(event `EnhancedInput|/Game/Project_ND/Character/Player_Input/IA_NDLook`
  (params (ActionValue :type "Vector2D Structure") (ElapsedSeconds :type "Float (double-precision)") (TriggeredSeconds :type "Float (double-precision)") (InputAction :type "InputAction Object Reference" :default "/Game/Project_ND/Character/Player_Input/IA_NDLook.IA_NDLook"))
  (:`Triggered`
    (`self.AddControllerYawInput` ActionValue_X)
    (`self.AddControllerPitchInput` (* ActionValue_Y -1.0))))

(event `EnhancedInput|/Game/Project_ND/Character/Player_Input/IA_NDSprint`
  (params (ActionValue :type Boolean) (ElapsedSeconds :type "Float (double-precision)") (TriggeredSeconds :type "Float (double-precision)") (InputAction :type "InputAction Object Reference" :default "/Game/Project_ND/Character/Player_Input/IA_NDSprint.IA_NDSprint"))
  (:`Ongoing`
    (set `CharacterMovementComponent.MaxWalkSpeed` 800.0 (`self.CharacterMovement`)))
  (:`Completed`
    (set `CharacterMovementComponent.MaxWalkSpeed` 600.0 (`self.CharacterMovement`))))

(event `EnhancedInput|/Game/Project_ND/Character/Player_Input/IA_NDWalk`
  (params (ActionValue :type Boolean) (ElapsedSeconds :type "Float (double-precision)") (TriggeredSeconds :type "Float (double-precision)") (InputAction :type "InputAction Object Reference" :default "/Game/Project_ND/Character/Player_Input/IA_NDWalk.IA_NDWalk"))
  (:`Started`
    (bind _output_get (set `self.isWalking` (not (`self.isWalking`))))
    (if _output_get
      (set `CharacterMovementComponent.MaxWalkSpeed` 400.0 (`self.CharacterMovement`))
      (else
        (set `CharacterMovementComponent.MaxWalkSpeed` 600.0 (`self.CharacterMovement`))))))

(event `EnhancedInput|/Game/Project_ND/Character/Player_Input/IA_NDJump`
  (params (ActionValue :type Boolean) (ElapsedSeconds :type "Float (double-precision)") (TriggeredSeconds :type "Float (double-precision)") (InputAction :type "InputAction Object Reference" :default "/Game/Project_ND/Character/Player_Input/IA_NDJump.IA_NDJump"))
  (:`Started`
    (`self.Jump`)))

(fn `UserConstructionScript`)