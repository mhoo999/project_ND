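; BP_NAdust is an actor that switches its Dust effect on and off based on player movement.
; Each Tick it casts the first player character to BPC_NDPlayerCharacter and reads velocity from that character's PlayerController, reached through PlayerState, rather than from the character itself.
; Dust activates while that speed exceeds a small threshold and deactivates otherwise.
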(event `self.ReceiveTick`
  (params (DeltaSeconds :type "Float (single-precision)"))
  (bind _asbpc_ndplayer_character (cast `/Game/Project_ND/Core/Character/BPC_NDPlayerCharacter` (`GameplayStatics.GetPlayerCharacter` 0)))
  (if (> (`KismetMathLibrary.VSize` (`self.GetVelocity` (`PlayerState.GetPlayerController` (`Pawn.PlayerState` _asbpc_ndplayer_character)))) 0.5)
    (`ActorComponent.Activate` (`self.dust`) false)
    (else
      (`ActorComponent.Deactivate` (`self.dust`)))))

(fn `UserConstructionScript`)