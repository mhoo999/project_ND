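; Lamp Blueprint that animates its spotlight and plays a sound while something overlaps its Box trigger.
; On Box overlap, it spawns the light sound at the actor if none is active and plays a Timeline that drives SpotLight intensity.
; Box exit destroys the sound and restores a fixed intensity, while actor-level end overlap stops the Timeline.
; Actor-level begin overlap stops a second Timeline that is never played here.
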(event `self.Box.OnComponentBeginOverlap`
  (params (OverlappedComponent :type "PrimitiveComponent Object Reference") (OtherActor :type "Actor Object Reference") (OtherComp :type "PrimitiveComponent Object Reference") (OtherBodyIndex :type Integer) (bFromSweep :type Boolean) (SweepResult :type "HitResult Structure (by ref)"))
  (`/Engine/EditorBlueprintResources/StandardMacros.IsValid` (`self.Sound`)
    (:`Is Valid`
      (bind (_direction `_새_트랙_0`) (`Timeline|타임라인` :!label _label)
        (:`Update`
          (`LightComponent.SetIntensity` (`self.SpotLight`) `_새_트랙_0`))))
    (:`Is Not Valid`
      (bind _returnvalue (`GameplayStatics.SpawnSoundAtLocation` "/Game/Project_ND/building/sound/SQ_lightASound.SQ_lightASound" (`self.K2_GetActorLocation`) (struct) 1.0 1.0 0.0 null null))
      (set `self.Sound` _returnvalue)
      (goto _label))))

(event `self.ReceiveActorEndOverlap`
  (params (OtherActor :type "Actor Object Reference"))
  (goto _label :!via `Stop`))

(event `self.ReceiveTick`
  (params (DeltaSeconds :type "Float (single-precision)")))

(event `self.Box.OnComponentEndOverlap`
  (params (OverlappedComponent :type "PrimitiveComponent Object Reference") (OtherActor :type "Actor Object Reference") (OtherComp :type "PrimitiveComponent Object Reference") (OtherBodyIndex :type Integer))
  (bind _sound (`self.Sound`))
  (`/Engine/EditorBlueprintResources/StandardMacros.IsValid` _sound
    (:`Is Valid`
      (`AudioComponent.Stop` _sound)
      (`ActorComponent.K2_DestroyComponent` _sound)
      (set `self.Sound` null)
      (`LightComponent.SetIntensity` (`self.SpotLight`) 20000.0))))

(event `self.ReceiveActorBeginOverlap`
  (params (OtherActor :type "Actor Object Reference"))
  (`Timeline|타임라인_0` :!via `Stop`))

(fn `UserConstructionScript`)