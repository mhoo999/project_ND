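; Player character Blueprint for Project_ND that adds a montage-backed flashlight toggle with sounds and a hold-and-release brick throw.
; Holding throw spawns a brick on the hand socket, and a montage notify starts the aiming state.
; While aiming, a self-re-calling delayed event redraws the predicted arc each frame as spline meshes.
; Releasing while aiming plays the throw-end section, then launches the brick after a short delay.
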(event `EnhancedInput|/Game/Project_ND/Character/Player_Input/IA_FlashLight`
  (params (ActionValue :type Boolean) (ElapsedSeconds :type "Float (double-precision)") (TriggeredSeconds :type "Float (double-precision)") (InputAction :type "InputAction Object Reference" :default "/Game/Project_ND/Character/Player_Input/IA_FlashLight.IA_FlashLight"))
  (bind _spotlight (`self.SpotLight`))
  (bind _returnvalue (`SceneComponent.K2_GetComponentLocation` _spotlight))
  (:`Triggered`
    (`|PlayMontage` (`self.Mesh`) "/Game/Project_ND/Character/CharacterAnim/NDPlayer_Montage/Standing_Taunt_Chest_fix_Montage.Standing_Taunt_Chest_fix_Montage"
      (:`then`
        (`/Engine/EditorBlueprintResources/StandardMacros.FlipFlop`
          (:`A`
            (`GameplayStatics.PlaySoundAtLocation` "/Engine/VREditor/Sounds/UI/Camera_Shutter.Camera_Shutter" _returnvalue (struct) 1.0 1.0 0.0 null null null null)
            (`KismetSystemLibrary.Delay` 1.0)
            (`SceneComponent.SetVisibility` _spotlight true false)
            (set `self.bFlahsLight` true))
          (:`B`
            (`GameplayStatics.PlaySoundAtLocation` "/Engine/VREditor/Sounds/UI/Click_on_Button.Click_on_Button" _returnvalue (struct) 1.0 1.0 0.0 null null null null)
            (`SceneComponent.SetVisibility` _spotlight false false)
            (set `self.bFlahsLight` false)))))))

(event `EnhancedInput|/Game/Project_ND/Character/Player_Input/IA_Throw`
  (params (ActionValue :type Boolean) (ElapsedSeconds :type "Float (double-precision)") (TriggeredSeconds :type "Float (double-precision)") (InputAction :type "InputAction Object Reference" :default "/Game/Project_ND/Character/Player_Input/IA_Throw.IA_Throw"))
  (bind _bp_throwable (`self.BP_Throwable`))
  (bind _returnvalue (`SceneComponent.GetSocketTransform` (`self.Mesh`) "Throw_Socket" "RTS_World"))
  (:`Triggered`
    (`|PlayMontage` (`self.Mesh`) "/Game/Project_ND/Character/CharacterAnim/NDPlayer_Montage/Throw1_Montage.Throw1_Montage"
      (:`then`
        (`KismetSystemLibrary.Delay` 0.2)
        (bind _returnvalue_2 (`|SpawnActorFromClass` "/Game/Project_ND/PickUpObject/Items/BP_Trowable_Brick.BP_Trowable_Brick_C" (`KismetMathLibrary.MakeTransform` (+ (.location _returnvalue) (20.0 0.0 0.0)) (`KismetMathLibrary.MakeRotator` (.roll (.rotation _returnvalue)) (- (.pitch (.rotation _returnvalue)) -180.0) (- (.yaw (.rotation _returnvalue)) 20.0)) (3.0 3.0 3.0)) "AdjustIfPossibleButAlwaysSpawn" "MultiplyWithRoot" null null))
        (bind _output_get (set `self.BP_Throwable` _returnvalue_2))
        (`self.K2_AttachToComponent` _output_get (`self.Mesh`) "Throw_Socket" "SnapToTarget" "SnapToTarget" "KeepWorld" false))
      (:`OnNotifyBegin`
        (set `self.Throwing` true)
        (`self.ShowProjectilePath`))))
  (:`Completed`
    (if (`self.Throwing`)
      (`|PlayMontage` (`self.Mesh`) "/Game/Project_ND/Character/CharacterAnim/NDPlayer_Montage/Throw1_Montage.Throw1_Montage" 1.0 0.0 "ThrowEnd"
        (:`then`
          (set `self.Throwing` false)
          (`KismetSystemLibrary.Delay` 0.4)
          (`/Engine/EditorBlueprintResources/StandardMacros.IsValid` _bp_throwable
            (:`Is Valid`
              (`/Game/Project_ND/PickUpObject/Items/BP_Trowable_Brick.Throw` _bp_throwable (`self.ThrowVelocity`))))))
      (else
        (`self.StopAnimMontage` "/Game/Project_ND/Character/CharacterAnim/NDPlayer_Montage/Throw1_Montage.Throw1_Montage")))))

(event `ShowProjectilePath`
  (bind _splinemeshcomponent (`self.SplineMeshComponent`))
  (bind _projectilepath (`self.ProjectilePath`))
  (`SplineComponent.ClearSplinePoints` (`self.ProjectilePath`) true)
  (for _array_element _splinemeshcomponent
    (`ActorComponent.K2_DestroyComponent` _array_element))
  (`KismetArrayLibrary.Array_Clear` _splinemeshcomponent)
  (if (`self.Throwing`)
    (bind (_outhit _outpathpositions) (`GameplayStatics.Blueprint_PredictProjectilePath_ByTraceChannel` (`SceneComponent.K2_GetComponentLocation` (`self.ProjectilStart`)) (`self.ThrowVelocity`) true 0.0 "ECC_Camera" false (`|MakeArray` self :!type "Actor Object Reference")))
    (for (_array_element_2 _array_index) _outpathpositions
      (`SplineComponent.AddSplinePointAtIndex` (`self.ProjectilePath`) _array_element_2 _array_index "Local" true))
    (for _index (range (+ (- (`SplineComponent.GetNumberOfSplinePoints` (`self.ProjectilePath`)) 2) 1))
      (bind _returnvalue (`AddComponent|NODE_AddSplineMeshComponent-0` :`bManualAttachment` true))
      (bind _returnvalue_2 (+ _index 1))
      (`SplineMeshComponent.SetStartAndEnd` _returnvalue (`SplineComponent.GetLocationAtSplinePoint` _projectilepath _index "Local") (`SplineComponent.GetTangentAtSplinePoint` _projectilepath _index "Local") (`SplineComponent.GetLocationAtSplinePoint` _projectilepath _returnvalue_2 "Local") (`SplineComponent.GetTangentAtSplinePoint` _projectilepath _returnvalue_2 "Local") true)
      (`KismetArrayLibrary.Array_Add` (`self.SplineMeshComponent`) _returnvalue))
    (`KismetSystemLibrary.Delay` (`GameplayStatics.GetWorldDeltaSeconds`))
    (`self.ShowProjectilePath`)))

(fn `UserConstructionScript`)